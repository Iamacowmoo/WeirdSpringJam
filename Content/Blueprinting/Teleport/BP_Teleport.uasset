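; BP_Teleport is a teleport pad that moves an overlapping BP_ThirdPersonCharacter to a linked pad and enables its shooting.
; BeginPlay finds pads by the LinkedPad tag; overlap uses the first, moving the player just above it after a brief delay.
; The source sets the destination's JustTriggered before the move to suppress re-triggering, then its EventLocked.
; End overlap clears JustTriggered only while EventLocked is false, then locks itself.
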(event `self.ReceiveBeginPlay`
  ;[1 1 1] Tag
  (bind _outactors (`GameplayStatics.GetAllActorsOfClassWithTag` "BP_Teleport_C" (`self.Linked Pad`)))
  (set `self.Pad Array` _outactors))

(event `self.Box.OnComponentBeginOverlap`
  (params (OverlappedComponent :type "PrimitiveComponent Object Reference") (OtherActor :type "Actor Object Reference") (OtherComp :type "PrimitiveComponent Object Reference") (OtherBodyIndex :type Integer) (bFromSweep :type Boolean) (SweepResult :type "HitResult Structure (by ref)"))
  (bind _output (`|GetArrayItem` (`self.Pad Array`)))
  ;[1 1 1] Teleport
  (bind _asbp_third_person_character (cast `/Game/ThirdPerson/Blueprints/BP_ThirdPersonCharacter` OtherActor))
  (set `self.Player_Ref` _asbp_third_person_character)
  (if (not (`self.Just Triggered`))
    (`/Engine/EditorBlueprintResources/StandardMacros.IsValid` _output
      (:`Is Valid`
        (set `/Game/Blueprinting/Teleport/BP_Teleport.Just Triggered` true _output)
        (`KismetSystemLibrary.Delay` 0.3)
        (`self.K2_SetActorRelativeLocation` (`self.Player_Ref`) (+ (`SceneComponent.RelativeLocation` (`/Game/Blueprinting/Teleport/BP_Teleport.DefaultSceneRoot` _output)) (0.0 0.0 100.0)) false false)
        (set `/Game/Blueprinting/Teleport/BP_Teleport.Event Locked` true _output)
        (set `/Game/ThirdPerson/Blueprints/BP_ThirdPersonCharacter.canShoot` true _asbp_third_person_character)))))

(event `self.Box.OnComponentEndOverlap`
  (params (OverlappedComponent :type "PrimitiveComponent Object Reference") (OtherActor :type "Actor Object Reference") (OtherComp :type "PrimitiveComponent Object Reference") (OtherBodyIndex :type Integer))
  ;[1 1 1] Once we teleport, we are ending the teleport
  (if (not (`self.Event Locked`))
    (set `self.Just Triggered` false)
    (set `self.Event Locked` true)))

(fn `UserConstructionScript`)